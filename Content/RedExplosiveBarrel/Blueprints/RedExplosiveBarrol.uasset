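; Red explosive barrel actor that catches fire when damaged and then explodes.
; Damage lowers its HP; at half health or below it starts burning and, after a short random delay, damages itself enough to detonate.
; Tick detects zero HP and triggers the explosion, which blackens and launches the mesh, plays effects and sound, and damages overlapping actors, firing a radial impulse per actor.
; The fire deactivates after a delay.
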(event `self.ReceiveBeginPlay`
  (set `self.HP` 200.0))

(event `self.ReceiveActorBeginOverlap`
  (params (OtherActor :type "Actor Object Reference")))

(event `self.ReceiveTick`
  (params (DeltaSeconds :type "Float (single-precision)"))
  (if (and (<= (`self.HP`) 0.0) (not (`self.isExploded`)))
    (`self.Epxlosion`)
    (`KismetSystemLibrary.Delay` 10.0)
    (`ActorComponent.Deactivate` (`self.Fire`))))

(event `self.ReceiveAnyDamage`
  (params (Damage :type "Float (single-precision)") (DamageType :type "DamageType Object Reference") (InstigatedBy :type "Controller Object Reference") (DamageCauser :type "Actor Object Reference"))
  (bind _output_get (set `self.HP` (- (`self.HP`) Damage)))
  (if (and (<= _output_get 100.0) (not (`self.isExploded`)))
    (`ActorComponent.Activate` (`self.Fire`) false)
    (`KismetSystemLibrary.Delay` (`KismetMathLibrary.RandomFloatInRange` 2.0 5.0))
    (`GameplayStatics.ApplyDamage` (`ActorComponent.GetOwner` (`self.Cylinder`)) 200.0)))

(fn `Epxlosion`
  (set `self.isExploded` true)
  (`ActorComponent.Activate` (`self.Explosion`) false)
  (`PrimitiveComponent.SetMaterial` (`self.Cylinder`) 0 "/Game/RedExplosiveBarrel/Materials/BlackBerrol.BlackBerrol")
  (`PrimitiveComponent.AddImpulse` (`self.Cylinder`) (`KismetMathLibrary.MakeVector` 0.0 (`KismetMathLibrary.RandomFloatInRange` 50000.0 100000.0) (`KismetMathLibrary.RandomFloatInRange` 500000.0 1000000.0)) "None" false)
  (`PrimitiveComponent.AddAngularImpulseInDegrees` (`self.Cylinder`) (`KismetMathLibrary.MakeVector` (`KismetMathLibrary.RandomFloatInRange` 100.0 200.0) (`KismetMathLibrary.RandomFloatInRange` 100.0 200.0) (`KismetMathLibrary.RandomFloatInRange` 100.0 200.0)) "None" true)
  (`GameplayStatics.PlaySoundAtLocation` "/Game/RedExplosiveBarrel/Audio/Explosion01.Explosion01" (`self.K2_GetActorLocation`) (struct) 1.0 1.0 0.0 null null null)
  (for _array_element (`PrimitiveComponent.GetOverlappingActors` (`self.DamageVolume`) "/Script/Engine.Actor")
    (`GameplayStatics.ApplyDamage` _array_element 150.0)
    (`RadialForceComponent.FireImpulse` (`self.RadialForce`))))

(fn `UserConstructionScript`)